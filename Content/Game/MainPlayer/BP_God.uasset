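; BP_God is a player pawn, apparently a free-moving overseer, moved with forward and right axis input along its root component's directions.
; On BeginPlay it finds the TopDownCharacter with CharacterID 999 if none is set, then calls the parent.
; The K key makes that character buy a hard-coded batch of peasant units, apparently as a test.
; Older manual camera movement and scroll-height logic remains disconnected; mouse axis events are empty.
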(event `self.ReceiveTick`
  (params (DeltaSeconds :type "Float (single-precision)")))

(event `self.ReceiveBeginPlay`
  (if (not (`KismetSystemLibrary.IsValid` (`self.PlayerCharacter`)))
    (bind _outactors (`GameplayStatics.GetAllActorsOfClass` "/Game/TopDownCPP/Blueprints/TopDownCharacter.TopDownCharacter_C"))
    (for _array_element _outactors
      (if (== (`TOLCharacter.CharacterID` _array_element) 999)
        (set `self.PlayerCharacter` _array_element))))
  (`parent.ReceiveBeginPlay`))

(event `Key|K` :consume false
  (params (Key :type "Key Structure"))
  (:`Pressed`
    (bind _astop_down_character (cast `/Game/TopDownCPP/Blueprints/TopDownCharacter` (`self.PlayerCharacter`)))
    (`/Game/TopDownCPP/Blueprints/TopDownCharacter.BuyUnitType` _astop_down_character "Peasants_01" 1150 100)))

(event `InputAxis|MoveForward`
  (params (AxisValue :type "Float (single-precision)"))
  (`self.AddMovementInput` (`SceneComponent.GetForwardVector` (`self.DefaultSceneRoot`)) AxisValue))

(event `InputAxis|MoveRight`
  (params (AxisValue :type "Float (single-precision)"))
  (`self.AddMovementInput` (`SceneComponent.GetRightVector` (`self.DefaultSceneRoot`)) AxisValue))

(event `InputAxis|MouseLookUp`
  (params (AxisValue :type "Float (single-precision)")))

(event `InputAxis|MouseLookRight`
  (params (AxisValue :type "Float (single-precision)")))

(event `InputAxis|MouseMiddleScroll`
  (params (AxisValue :type "Float (single-precision)")))

(event `InputAction|MouseMiddleClick`
  (params (Key :type "Key Structure")))

(fn `UserConstructionScript`)