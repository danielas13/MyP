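; Settlement actor that opens a settlement UI on interaction and tracks its own recruitment level.
; Construction loads its information from DT_SettlementInformation by SettlementID.
; Interaction checks and clears the GameMode's character-on-map message, then shows a cached widget, created on first use with that information.
; UpdateTOLSettlement, while below recruitment capacity, raises the level only when its timer is zero, otherwise increments the timer.
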(event `/Game/Game/Structures/BPI/BPI_IS_Interaction.IS_Interact`
  (params (Instigator :type "Actor Object Reference"))
  (bind _returnvalue (`GameplayStatics.GetGameMode`))
  (bind _isplayeronmainmap (message `/Game/Game/Structures/BPI/BPI_GM.GM_IsCharacterOnMap` _returnvalue))
  (if _isplayeronmainmap
    (message `/Game/Game/Structures/BPI/BPI_GM.GM_SetCharacterMap` _returnvalue false)
    (if (not (`KismetSystemLibrary.IsValid` (`self.SettlementUI`)))
      (bind _returnvalue_2 (`|CreateWidget` "/Game/Game/GameSystems/Settlements/SettlementUI/SettlementUI.SettlementUI_C"))
      (bind _output_get (set `self.SettlementUI` _returnvalue_2))
      (set `/Game/Game/GameSystems/Settlements/SettlementUI/SettlementUI.SettlementInfo` (`self.SettlementInformation`) _output_get))
    (set `/Game/Game/GameSystems/Settlements/SettlementUI/SettlementUI.OwningSettlement` self _output_get)
    (`UserWidget.AddToViewport` (`self.SettlementUI`) 0)))

(fn `UpdateTOLSettlement`
  (if (< (`self.CurrentReqruitmentLevel`) (`self.ReqruitmentCapacity`))
    (if (== (`self.TimeUntillReqruitmentUpdate`) 0)
      (set `self.CurrentReqruitmentLevel` (+ (`self.CurrentReqruitmentLevel`) 1))
      (set `self.TimeUntillReqruitmentUpdate` (`KismetMathLibrary.Abs_Int` 1))
      (else
        (set `self.TimeUntillReqruitmentUpdate` (+ (`self.TimeUntillReqruitmentUpdate`) 1))))))

(fn `UserConstructionScript`
  (bind _returnvalue (`|GetDataTableRow` "/Game/Game/Structures/DataTables/DT_SettlementInformation.DT_SettlementInformation" (`KismetStringLibrary.Conv_StringToName` (`KismetStringLibrary.Conv_IntToString` (`self.SettlementID`))))
    (:`then`
      (set `self.SettlementInformation` _returnvalue))))